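; BP_HttpServerInstance brings up an HTTP server, only when running as the server.
; On AfterInit it checks that the HTTP system is valid, then constructs a handler object from each class in InitHandleList.
; Each valid handler is registered as a route and stored in ArrayHandles, after which the server starts.
; An invalid system or failed construction only prints a message.
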(event EventAfterInit
  (bind _returnvalue (Subsystems|GetBPHttpSystem))
  (if (Networking|IsServer)
    (Utilities|IsValid _returnvalue
      (:Is%20Valid
        (Utilities|FlowControl|Sequence
          (:then_0
            (bind _result (Utilities|Set|ToArray (Variables|Default|GetinitHandleList)))
            (for _array_element _result
              (bind _returnvalue_2 (Game|ConstructObjectfromClass _array_element self))
              (Utilities|IsValid _returnvalue_2
                (:Is%20Valid
                  (Class|HttpSubsystem|AddRoute _returnvalue _returnvalue_2)
                  (Utilities|Array|Add (Variables|Default|GetarrayHandles) _returnvalue_2))
                (:Is%20Not%20Valid
                  (Development|PrintString "fail")))))
          (:then_1
            (Class|HttpSubsystem|StartServer _returnvalue)
            (Development|PrintString "Start Http Server"))))
      (:Is%20Not%20Valid
        (Development|PrintString "http system not valid")))))